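; Player controller Blueprint that owns the player's HUD and pause menu widgets.
; On BeginPlay it adds both widgets to the viewport with the menu hidden, passes itself to the menu and stores the viewport center.
; The Pause input calls TogglePauseMenu, which swaps widget visibility and switches game pause, input mode and cursor display.
; Each toggle also recenters the mouse on the stored position.
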(event EventBeginPlay
  (bind (_sizex _sizey) (HUD|GetViewportSize))
  (bind _returnvalue (UserInterface|CreateWidget "/Game/wHUD.wHUD_C"))
  (bind _output_get (Variables|Default|SetHUDRef _returnvalue))
  (UserInterface|Viewport|AddtoViewport _output_get 0)
  (bind _returnvalue_2 (UserInterface|CreateWidget "/Game/wPauseMenu.wPauseMenu_C"))
  (bind _output_get_2 (Variables|Default|SetPauseMenuRef _returnvalue_2))
  (Variables|/Game/wPauseMenu.wPauseMenu_C|SetPlayerControllerReference _output_get_2 self)
  (Widget|SetVisibility _output_get_2 "Hidden")
  (UserInterface|Viewport|AddtoViewport _output_get_2 0)
  (Variables|Default|SetPosX (/ _sizex 2))
  (Variables|Default|SetPosY (/ _sizey 2)))

(event EventTick
  (params (DeltaSeconds :type Float%20%28single-precision%29)))

(event Input|ActionEvents|InputActionPause
  (params (Key :type Key%20Structure))
  (:Pressed
    (CallFunction|TogglePauseMenu)))

(fn ConstructionScript)

(fn TogglePauseMenu
  (bind _self self)
  (bind _pausemenuref (Variables|Default|GetPauseMenuRef))
  (bind _hudref (Variables|Default|GetHUDRef))
  (if (Variables|Default|GetIsVisible)
    (Widget|SetVisibility _hudref "Visible")
    (Widget|SetVisibility _pausemenuref "Hidden")
    (Input|SetInputModeGameOnly _self)
    (bind _output_get (Variables|Default|SetIsVisible false))
    (Game|SetGamePaused _output_get)
    (Variables|/Script/Engine.PlayerController|SetbShowMouseCursor _self false)
    (else
      (Widget|SetVisibility _hudref "Hidden")
      (Widget|SetVisibility _pausemenuref "Visible")
      (Input|SetInputModeGameandUI _self _pausemenuref "LockAlways" true)
      (bind _output_get_2 (Variables|Default|SetIsVisible true))
      (Game|SetGamePaused _output_get_2)
      (Variables|/Script/Engine.PlayerController|SetbShowMouseCursor _self true)))
  (Class|PlayerController|SetMouseLocation (Variables|Default|GetPosX) (Variables|Default|GetPosY))
  (return))